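; BP_Monster05 is a monster Blueprint that carries a child actor, presumably its weapon, on its skeletal mesh.
; On BeginPlay it snaps the ChildActor component to the SKT_Weapon socket of Mesh.
; An unconnected roaming chain (random delay, AIMoveTo a random reachable nearby point, toggling IsMoving) never runs.
; Tick, overlap and the construction script are empty.
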(event EventBeginPlay
  (Transformation|AttachComponentToComponent (Variables|Default|GetChildActor) (Variables|Character|GetMesh) "SKT_Weapon" "SnapToTarget" "SnapToTarget" "SnapToTarget" true))

(event Collision|EventActorBeginOverlap
  (params (OtherActor :type Actor%20Object%20Reference)))

(event EventTick
  (params (DeltaSeconds :type Float%20%28single-precision%29)))

(fn ConstructionScript)