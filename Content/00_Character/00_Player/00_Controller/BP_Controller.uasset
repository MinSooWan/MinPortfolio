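; BP_Controller is a player controller Blueprint that seeds the player's inventory with starting items.
; On BeginPlay it spawns one tool, armor, weapon and recovery item actor in turn, adding each to the InventoryComp of player 0's PlayerCharacter.
; The item classes are hard-coded in the event graph, and Tick and the construction script do nothing.
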(event EventBeginPlay
  (bind _returnvalue (Game|GetPlayerCharacter 0))
  (bind _spawn_transform (Variables|Default|GetSpawn%20Transform))
  (bind _asplayer_character (Utilities|Casting|CastToPlayerCharacter _returnvalue))
  (bind _inventorycomp (Variables|/Script/MinPortfolio.PlayerCharacter|GetinventoryComp _asplayer_character))
  (bind _returnvalue_2 (Game|SpawnActorfromClass "/Game/01_Item/03_Tool/BP_Tool02.BP_Tool02_C" _spawn_transform "Undefined" 0 0))
  (Class|InventoryComponent|AddItem _inventorycomp _returnvalue_2)
  (bind _returnvalue_3 (Game|SpawnActorfromClass "/Game/01_Item/01_Armor/BP_Armor01.BP_Armor01_C" _spawn_transform "Undefined" 0 0))
  (Class|InventoryComponent|AddItem _inventorycomp _returnvalue_3)
  (bind _returnvalue_4 (Game|SpawnActorfromClass "/Game/01_Item/00_Weapon/BP_Weapon01.BP_Weapon01_C" _spawn_transform "Undefined" 0 0))
  (Class|InventoryComponent|AddItem _inventorycomp _returnvalue_4)
  (bind _returnvalue_5 (Game|SpawnActorfromClass "/Game/01_Item/04_BattleItem/Recover/BP_Recovery01.BP_Recovery01_C" _spawn_transform "Undefined" 0 0))
  (Class|InventoryComponent|AddItem _inventorycomp _returnvalue_5))

(event EventTick
  (params (DeltaSeconds :type Float%20%28single-precision%29)))

(fn ConstructionScript)